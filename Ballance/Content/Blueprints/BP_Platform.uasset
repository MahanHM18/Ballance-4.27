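; BP_Platform is an actor that the player tilts with the mouse.
; MouseX adds to its roll, clamped to plus or minus 90 degrees, and MouseY adds to its pitch within a narrower clamp.
; Each axis event reads the current rotation and sets it directly, preserving the other two components, with no sensitivity or delta-time scaling.
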(event `InputAxis|MouseX`
  (params (AxisValue :type "Float (single-precision)"))
  (`self.K2_SetActorRotation` (`KismetMathLibrary.MakeRotator` (`KismetMathLibrary.FClamp` (+ AxisValue (.roll (`self.K2_GetActorRotation`))) -90.0 90.0) (.pitch (`self.K2_GetActorRotation`)) (.yaw (`self.K2_GetActorRotation`)))))

(event `InputAxis|MouseY`
  (params (AxisValue :type "Float (single-precision)"))
  (`self.K2_SetActorRotation` (`KismetMathLibrary.MakeRotator` (.roll (`self.K2_GetActorRotation`)) (`KismetMathLibrary.FClamp` (+ AxisValue (.pitch (`self.K2_GetActorRotation`))) -60.0 60.0) (.yaw (`self.K2_GetActorRotation`)))))

(fn `UserConstructionScript`)