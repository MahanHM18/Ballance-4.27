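; BP_MainPlayerController is a player controller that tracks collected coins against a maximum and shows the count on the HUD.
; On BeginPlay it creates the player widget, adds it to the viewport, keeps a reference and refreshes the text.
; IncreaseCoin and IncreaseMaxCoin each bump their counter and call UpdateWidget, which writes the current and maximum values to the widget if it is valid.
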(event `self.ReceiveBeginPlay`
  (bind _returnvalue (`|CreateWidget` "/Game/Widgets/Widget_Player.Widget_Player_C"))
  (`UserWidget.AddToViewport` _returnvalue 0)
  (set `self.PlayerWidget` _returnvalue)
  (`self.UpdateWidget`))

(fn `IncreaseCoin`
  (`/Engine/EditorBlueprintResources/StandardMacros.IncrementInt` (`self.Coin`)
    (:`  `
      (`self.UpdateWidget`))))

(fn `IncreaseMaxCoin`
  (`/Engine/EditorBlueprintResources/StandardMacros.IncrementInt` (`self.MaxCoin`)
    (:`  `
      (`self.UpdateWidget`))))

(fn `UpdateWidget`
  (bind _playerwidget (`self.PlayerWidget`))
  (`/Engine/EditorBlueprintResources/StandardMacros.IsValid` _playerwidget
    (:`Is Valid`
      (`/Game/Widgets/Widget_Player.SetCoinText` _playerwidget (`KismetStringLibrary.Concat_StrStr` (`KismetStringLibrary.Conv_IntToString` (`self.Coin`)) " / " (`KismetStringLibrary.Conv_IntToString` (`self.MaxCoin`)))))))

(fn `UserConstructionScript`)